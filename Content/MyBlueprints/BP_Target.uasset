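; BP_Target is a shootable target that the first-person projectile damages and destroys.
; It registers itself with BP_GameMode through AddTarget on BeginPlay.
; Each projectile hit subtracts a fixed amount of Health, and other hits are ignored.
; When Health runs out, the actor destroys itself and calls RemoveTarget on the game mode.
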(event EventBeginPlay
  (bind _asbp_game_mode (Utilities|Casting|CastToBP_GameMode (Game|GetGameMode)))
  (Default|AddTarget _asbp_game_mode))

(event Collision|EventActorBeginOverlap
  (params (OtherActor :type Actor%20Object%20Reference)))

(event Collision|EventHit
  (params (MyComp :type Primitive%20Component%20Object%20Reference) (Other :type Actor%20Object%20Reference) (OtherComp :type Primitive%20Component%20Object%20Reference) (bSelfMoved :type Boolean) (HitLocation :type Vector :default "0, 0, 0") (HitNormal :type Vector :default "0, 0, 0") (NormalImpulse :type Vector :default "0, 0, 0") (Hit :type Hit%20Result%20Structure%20%28by%20ref%29))
  (Utilities|Casting|CastToBP_FirstPersonProjectile Other)
  (bind _output_get (Variables|Default|SetHealth (- (Variables|Default|GetHealth) 25)))
  (if (<= _output_get 0)
    (Actor|DestroyActor)
    (bind _asbp_game_mode (Utilities|Casting|CastToBP_GameMode (Game|GetGameMode)))
    (Default|RemoveTarget _asbp_game_mode)))

(fn ConstructionScript)