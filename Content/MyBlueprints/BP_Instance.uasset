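; BP_Instance is a game instance style Blueprint that handles level progression through an ordered Levels array.
; On Init it looks up the current level name in that array and stores its position as LevelIndex.
; ReloadLevel reopens the current level by name, while LoadNextLevel advances the index, wraps to the first entry after the last, and opens that level.
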(event EventInit
  (bind _returnvalue (Game|GetCurrentLevelName true))
  (if (>= (Utilities|Array|FindItem (Variables|Default|GetLevels) (Utilities|String|StringToName _returnvalue)) 0)
    (Variables|Default|SetLevel%20Index (Utilities|Array|FindItem (Variables|Default|GetLevels) (Utilities|String|StringToName _returnvalue)))))

(fn ReloadLevel
  (bind _returnvalue (Game|GetCurrentLevelName true))
  (Game|OpenLevel(byName) (Utilities|String|StringToName _returnvalue)))

(fn LoadNextLevel
  (if (>= (+ (Variables|Default|GetLevel%20Index) 1) (Utilities|Array|Length (Variables|Default|GetLevels)))
    (Variables|Default|SetLevel%20Index 0)
    (else
      (Variables|Default|SetLevel%20Index (+ (Variables|Default|GetLevel%20Index) 1))))
  (Game|OpenLevel(byName) (Utilities|Array|Get(acopy) (Variables|Default|GetLevels) (Variables|Default|GetLevel%20Index))))