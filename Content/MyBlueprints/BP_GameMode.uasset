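; BP_GameMode is a game mode that tracks how many targets remain in the level and advances to the next level when none are left.
; AddTarget increments TargetCount and RemoveTarget decrements it.
; When the count reaches zero or below, RemoveTarget casts the game instance to BP_Instance and calls LoadNextLevel.
; The event graph and construction script contain no logic.
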(event EventBeginPlay)

(event EventTick
  (params (DeltaSeconds :type Float%20%28single-precision%29)))

(fn ConstructionScript)

(fn AddTarget
  (Variables|Default|SetTarget%20Count (+ (Variables|Default|GetTarget%20Count) 1)))

(fn RemoveTarget
  (bind _output_get (Variables|Default|SetTarget%20Count (- (Variables|Default|GetTarget%20Count) 1)))
  (if (<= _output_get 0)
    (bind _asbp_instance (Utilities|Casting|CastToBP_Instance (Game|GetGameInstance)))
    (Default|LoadNextLevel _asbp_instance)))