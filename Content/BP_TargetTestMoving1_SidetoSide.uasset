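; A moving target actor that shuttles back and forth and is destroyed by two Projectile overlaps.
; Tick offsets it along normalized Direction by Speed without delta-time scaling, while a looping TimeToChange timer flips Direction.
; The first hit swaps the mesh material; the second spawns an explosion effect and sound, calls the TargetDestroyed dispatcher and destroys the actor.
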(event Custom|CustomEvent
  ;[1 1 1] Target Reverse Movement
  (Variables|Default|SetDirection (* (Variables|Default|GetDirection) -1.0)))

(event Collision|EventActorBeginOverlap
  (params (OtherActor :type Actor%20Object%20Reference))
  (bind _returnvalue (Transformation|GetActorLocation))
  (Utilities|Casting|CastToProjectile OtherActor)
  (bind _output_get (Variables|Default|SetState (+ (Variables|Default|GetState) 1)))
  (switch int _output_get
    (:1
      (Rendering|Material|SetMaterial (Variables|Default|GetStaticMesh) 0 "/Game/Mat_Target_Second.Mat_Target_Second"))
    (:2
      (Effects|SpawnEmitteratLocation "/Game/StarterContent/Particles/P_Explosion.P_Explosion" _returnvalue)
      (Audio|PlaySoundatLocation "/Game/StarterContent/Audio/Explosion02.Explosion02" _returnvalue "0, 0, 0" 1.0 1.0 0.0 0 0 0 0)
      (Default|CallTargetDestroyed)
      (Actor|DestroyActor))))

(event EventTick
  (params (DeltaSeconds :type Float%20%28single-precision%29))
  ;[1 1 1] Target Movement and Speed
  (Transformation|AddActorWorldOffset (* (Math|Vector|Normalize (Variables|Default|GetDirection)) (Variables|Default|GetSpeed))))

(event EventBeginPlay
  ;[1 1 1] Target Reverse Movement
  (Utilities|Time|SetTimerbyEvent (delegate Custom|CustomEvent) (Variables|Default|GetTime%20to%20Change) true))

(fn ConstructionScript)